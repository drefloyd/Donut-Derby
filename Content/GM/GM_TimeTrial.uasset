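; Time trial race game mode that tracks completed laps against a required count and ends the race with a win screen.
; On begin play and on each UpdateLaps call, it refreshes the lap counter text through LapsAsText.
; Once completed laps exceed the required count, it flags the race complete, shows the RaceWon widget, enables the cursor with UI-only input and pauses the game.
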(event `self.ReceiveBeginPlay`
  (set `self.LapsText` (`self.Laps As Text` (`self.LapsCompleted`) (`self.LapsRequired`))))

(event `Update Laps`
  (bind _returnvalue (`GameplayStatics.GetPlayerController` 0))
  (bind _lapsrequired (`self.LapsRequired`))
  (bind _lapscompleted (`self.LapsCompleted`))
  (set `self.LapsText` (`self.Laps As Text` _lapscompleted _lapsrequired))
  (if (> _lapscompleted _lapsrequired)
    (set `self.raceComplete` true)
    (bind _returnvalue_2 (`|CreateWidget` "/Game/UI/RaceWon_WB.RaceWon_WB_C"))
    (`UserWidget.AddToViewport` _returnvalue_2 0)
    (set `PlayerController.bShowMouseCursor` true _returnvalue)
    (`WidgetBlueprintLibrary.SetInputMode_UIOnlyEx` _returnvalue null)
    (`GameplayStatics.SetGamePaused` true)))

(fn `UserConstructionScript`)