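; AI start/finish line trigger that counts a rival donut's laps and ends the race as a loss for the player.
; The first AI_Donut to overlap the Cube is flagged as the rival, and only its crossings increment the lap count.
; On the fourth crossing it shows the RaceLost_WB widget, enables the cursor with UI-only input and pauses the game.
; Overlaps by other actor types print an error.
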(event `self.Cube.OnComponentBeginOverlap`
  (params (OverlappedComponent :type "PrimitiveComponent Object Reference") (OtherActor :type "Actor Object Reference") (OtherComp :type "PrimitiveComponent Object Reference") (OtherBodyIndex :type Integer) (bFromSweep :type Boolean) (SweepResult :type "HitResult Structure (by ref)"))
  (bind _ailaps (`self.AiLaps`))
  ;[1 1 1] When start/finish line is crossed by Ai
  (bind _asai_donut (cast `/Game/VehicleTemplate/Blueprints/SportsCar/AI_Donut` OtherActor)
    (:`then`
      (if (not (`self.RivalPicked`))
        (set `/Game/VehicleTemplate/Blueprints/SportsCar/AI_Donut.Is_Rival` true _asai_donut)
        (set `self.RivalPicked` true))
      (if (`/Game/VehicleTemplate/Blueprints/SportsCar/AI_Donut.Is_Rival` _asai_donut)
        (set `self.AiLaps` (+ 1 _ailaps))
        (if (== 4 _ailaps)
          (bind _returnvalue (`|CreateWidget` "/Game/UI/RaceLost_WB.RaceLost_WB_C"))
          (`UserWidget.AddToViewport` _returnvalue 0)
          (set `PlayerController.bShowMouseCursor` true (`GameplayStatics.GetPlayerController` 0))
          (`WidgetBlueprintLibrary.SetInputMode_UIOnlyEx` null null)
          (`GameplayStatics.SetGamePaused` true))))
    (:`CastFailed`
      (`KismetSystemLibrary.PrintText` "ERROR"))))

(fn `UserConstructionScript`
  (set `self.RivalPicked` false))