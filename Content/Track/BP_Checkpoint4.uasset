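; BP_Checkpoint4 is a track checkpoint that records on the start line that checkpoint 4 has been passed.
; Overlapping either its Cube or its JumpCollider hides the checkpoint, reveals the StartLine actor and sets CheckPoint4Passed on it through a BP_StartLine cast.
; The player-name checks meant to ignore AI cars are disconnected, so any overlapping actor triggers it.
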(event `self.Cube.OnComponentBeginOverlap`
  (params (OverlappedComponent :type "PrimitiveComponent Object Reference") (OtherActor :type "Actor Object Reference") (OtherComp :type "PrimitiveComponent Object Reference") (OtherBodyIndex :type Integer) (bFromSweep :type Boolean) (SweepResult :type "HitResult Structure (by ref)"))
  (bind _startline (`self.StartLine`))
  ;[1 1 1] When start/finish line is crossed
  (`self.SetActorHiddenInGame` true :!label _label)
  (`self.SetActorHiddenInGame` _startline false)
  (bind _asbp_start_line (cast `/Game/Track/BP_StartLine` _startline))
  (set `/Game/Track/BP_StartLine.CheckPoint4Passed` true _asbp_start_line))

(event `self.JumpCollider.OnComponentBeginOverlap`
  (params (OverlappedComponent :type "PrimitiveComponent Object Reference") (OtherActor :type "Actor Object Reference") (OtherComp :type "PrimitiveComponent Object Reference") (OtherBodyIndex :type Integer) (bFromSweep :type Boolean) (SweepResult :type "HitResult Structure (by ref)"))
  ;[1 1 1] When start/finish line is crossed
  (goto _label))

(fn `UserConstructionScript`)