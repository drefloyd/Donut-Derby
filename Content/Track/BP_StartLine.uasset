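; BP_StartLine is the time-trial start/finish line that starts the race and counts laps.
; Overlapping its Cube or JumpCollider hides the line and reveals Checkpoint1; the first crossing starts the lap timer and race through the VehiclePlayerController.
; Later crossings count a lap in GM_TimeTrial and restart the lap only if CheckPoint4Passed is set, then clear that flag.
; The pawn-name checks meant to ignore AI are disconnected, so any overlapping actor triggers it.
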(event `self.ReceiveBeginPlay`
  (bind _asvehicle_player_controller (cast `/Game/VehicleTemplate/Blueprints/VehiclePlayerController` (`GameplayStatics.GetPlayerController` 0)))
  (set `self.As Vehicle Player Controller` _asvehicle_player_controller)
  (bind _asgm_time_trial (cast `/Game/GM/GM_TimeTrial` (`GameplayStatics.GetGameMode`)))
  (set `self.As GM Time Trial` _asgm_time_trial))

(event `self.Cube.OnComponentBeginOverlap`
  (params (OverlappedComponent :type "PrimitiveComponent Object Reference") (OtherActor :type "Actor Object Reference") (OtherComp :type "PrimitiveComponent Object Reference") (OtherBodyIndex :type Integer) (bFromSweep :type Boolean) (SweepResult :type "HitResult Structure (by ref)"))
  (bind _as_gm_time_trial (`self.As GM Time Trial`))
  (bind _as_vehicle_player_controller (`self.As Vehicle Player Controller`))
  ;[1 1 1] When start/finish line is crossed
  (`self.SetActorHiddenInGame` true :!label _label)
  (`self.SetActorHiddenInGame` (`self.Checkpoint1`) false)
  (if (`self.raceStarted`)
    (if (`self.CheckPoint4Passed`)
      (`/Engine/EditorBlueprintResources/StandardMacros.IncrementInt` (`/Game/GM/GM_TimeTrial.LapsCompleted` _as_gm_time_trial)
        (:`  `
          (`/Game/VehicleTemplate/Blueprints/VehiclePlayerController.StartLap` (`self.As Vehicle Player Controller`))
          (`/Game/GM/GM_TimeTrial.Update Laps` _as_gm_time_trial)
          (set `self.CheckPoint4Passed` false))))
    (else
      (`/Game/VehicleTemplate/Blueprints/VehiclePlayerController.StartLap` _as_vehicle_player_controller)
      (`/Engine/EditorBlueprintResources/StandardMacros.DoOnce` false
        (:`Completed`
          (`/Game/VehicleTemplate/Blueprints/VehiclePlayerController.Start Race` _as_vehicle_player_controller)
          (set `self.raceStarted` true)
          (`/Engine/EditorBlueprintResources/StandardMacros.DecrementFloat` (`KismetMathLibrary.Conv_IntToDouble` (`/Game/GM/GM_TimeTrial.LapsCompleted` (`self.As GM Time Trial`)))))))))

(event `self.JumpCollider.OnComponentBeginOverlap`
  (params (OverlappedComponent :type "PrimitiveComponent Object Reference") (OtherActor :type "Actor Object Reference") (OtherComp :type "PrimitiveComponent Object Reference") (OtherBodyIndex :type Integer) (bFromSweep :type Boolean) (SweepResult :type "HitResult Structure (by ref)"))
  ;[1 1 1] When start/finish line is crossed
  (goto _label))

(fn `UserConstructionScript`)